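; BP_ActivarPuerta is an interactable quest door that opens only while the quest is In Progress.
; A box overlap with the third-person character toggles a Spanish text prompt, either asking to start the mission or to press E.
; Interact calls OpenDoor, which notifies QuestManager1111 and plays a Timeline that offsets the mesh vertically from its BeginPlay location.
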(event OnComponentBeginOverlap(Box)
  (params (OverlappedComponent :type Primitive%20Component%20Object%20Reference) (OtherActor :type Actor%20Object%20Reference) (OtherComp :type Primitive%20Component%20Object%20Reference) (OtherBodyIndex :type Integer) (bFromSweep :type Boolean) (SweepResult :type Hit%20Result%20Structure%20%28by%20ref%29))
  (bind _textrender (Variables|Default|GetTextRender))
  (Utilities|Casting|CastToBP_ThirdPersonCharacter OtherActor)
  (Rendering|SetVisibility (Variables|Default|GetTextRender) true false)
  (switch Utilities|FlowControl|Switch|SwitchonEQuestState (Variables|/Game/QuestSystem/BP_QuestManager.BP_QuestManager_C|GetEQuestState (Variables|Default|GetQuestManager1111))
    (:NewEnumerator0
      (Rendering|Components|TextRender|SetText _textrender (Utilities|Text|MakeLiteralText "Tienes que empezar <br> primero la mision")))
    (:NewEnumerator1
      (Rendering|Components|TextRender|SetText _textrender (Utilities|Text|MakeLiteralText "Pulsa E <br> para interactuar")))))

(event OnComponentEndOverlap(Box)
  (params (OverlappedComponent :type Primitive%20Component%20Object%20Reference) (OtherActor :type Actor%20Object%20Reference) (OtherComp :type Primitive%20Component%20Object%20Reference) (OtherBodyIndex :type Integer))
  (bind _textrender (Variables|Default|GetTextRender))
  (Utilities|Casting|CastToBP_ThirdPersonCharacter OtherActor)
  (Rendering|SetVisibility (Variables|Default|GetTextRender) false false)
  (switch Utilities|FlowControl|Switch|SwitchonEQuestState (Variables|/Game/QuestSystem/BP_QuestManager.BP_QuestManager_C|GetEQuestState (Variables|Default|GetQuestManager1111))
    (:NewEnumerator0
      (Rendering|Components|TextRender|SetText _textrender (Utilities|Text|MakeLiteralText "Tienes que empezar <br> primero la mision")))
    (:NewEnumerator1
      (Rendering|Components|TextRender|SetText _textrender (Utilities|Text|MakeLiteralText "Pulsa E <br> para interactuar")))))

(event Custom|Open%20Door
  (switch Utilities|FlowControl|Switch|SwitchonEQuestState (Variables|/Game/QuestSystem/BP_QuestManager.BP_QuestManager_C|GetEQuestState (Variables|Default|GetQuestManager1111))
    (:NewEnumerator1
      (Default|DoorOpened (Variables|Default|GetQuestManager1111))
      (bind _newtrack_0 (Timeline|Timeline Play)
        (:Update
          (Transformation|SetWorldLocation (Variables|Debug|GetStaticMeshComponent) (+ (Variables|Default|GetLocalizacionInicio) (Math|Vector|MakeVector 0.0 0.0 _newtrack_0)) false false))))))

(event EventBeginPlay
  (Variables|Default|SetLocalizacionInicio (Transformation|GetWorldLocation (Variables|Debug|GetStaticMeshComponent))))

(fn ConstructionScript)

(fn Interact
  (CallFunction|OpenDoor)
  (return true))