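; BP_QuestManager is an interactable quest-giver that tracks a quest to collect objects and open a door.
; Interacting starts the quest, creating the QuestScreen widget and counting ObjectToFind actors, or completes it once objectives are done.
; Collection and door events refresh the widget, check completion and update Spanish TextRender prompts.
; A bridge objective flag is set by event but affects neither completion nor the widget.
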(event Custom|Door%20Opened
  (Variables|Default|SetOpenDoorObjective true)
  (CallFunction|UpdateQuestText)
  (if (and (== (Variables|Default|GetObjectsCollected) (Variables|Default|GetTotalObjectsToCollect)) (Variables|Default|GetOpenDoorObjective))
    (Variables|Default|SetEQuestState "NewEnumerator2")
    (Rendering|Components|TextRender|SetText (Variables|Default|GetTextRender) (Utilities|Text|MakeLiteralText "Presiona \"E\" para <br>completar la misión"))))

(event Custom|Start_Interaction
  (switch Utilities|FlowControl|Switch|SwitchonEQuestState (Variables|Default|GetEQuestState)
    (:NewEnumerator0
      (Utilities|FlowControl|Sequence
        (:then_0
          (Variables|Default|SetEQuestState "NewEnumerator1")
          (bind _returnvalue (UserInterface|CreateWidget "/Game/QuestSystem/QuestScreen.QuestScreen_C"))
          (bind _output_get (Variables|Default|SetQuestWidget _returnvalue))
          (UserInterface|Viewport|AddtoViewport _output_get 0))
        (:then_1
          (bind _outactors (Actor|GetAllActorsOfClass "/Game/QuestSystem/ObjectToFind.ObjectToFind_C"))
          (Variables|Default|SetTotalObjectsToCollect (Utilities|Array|Length _outactors)))
        (:then_2
          (CallFunction|UpdateQuestText)
          (Rendering|Components|TextRender|SetText (Variables|Default|GetTextRender) (Utilities|Text|MakeLiteralText "Regresa cuando <br>Termines las misiones")))))
    (:NewEnumerator2
      (Variables|Default|SetEQuestState "NewEnumerator3")
      (Widget|RemovefromParent (Variables|Default|GetQuestWidget))
      (Rendering|Components|TextRender|SetText (Variables|Default|GetTextRender) (Utilities|Text|MakeLiteralText "MISION COMPLETADA")))))

(event Custom|UpdateQuestText
  (Variables|/Game/QuestSystem/QuestScreen.QuestScreen_C|SetCoinSignsFound (Variables|Default|GetQuestWidget) (Variables|Default|GetObjectsCollected))
  (Variables|/Game/QuestSystem/QuestScreen.QuestScreen_C|SetTotalNumberOfCoinsSings (Variables|Default|GetQuestWidget) (Variables|Default|GetTotalObjectsToCollect))
  (Variables|/Game/QuestSystem/QuestScreen.QuestScreen_C|SetDoorOpened (Variables|Default|GetQuestWidget) (Variables|Default|GetOpenDoorObjective)))

(event Custom|Add%20Object%20Found
  (Math|Integer|IncrementInt (Variables|Default|GetObjectsCollected)
    (:%20%20
      (CallFunction|UpdateQuestText)
      (if (and (== (Variables|Default|GetObjectsCollected) (Variables|Default|GetTotalObjectsToCollect)) (Variables|Default|GetOpenDoorObjective))
        (Variables|Default|SetEQuestState "NewEnumerator2")
        (Rendering|Components|TextRender|SetText (Variables|Default|GetTextRender) (Utilities|Text|MakeLiteralText "Presiona \"E\" para <br>completar la misión"))))))

(event Custom|Bridge%20Objective
  (Variables|Default|SetBridgeObjective true))

(event EventBeginPlay)

(event Collision|EventActorBeginOverlap
  (params (OtherActor :type Actor%20Object%20Reference)))

(event EventTick
  (params (DeltaSeconds :type Float%20%28single-precision%29)))

(fn ConstructionScript)

(fn Interact
  (CallFunction|StartInteraction)
  (return true))