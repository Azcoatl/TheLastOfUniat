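; BP_EnemyMelee2 is an enemy Blueprint that roams between random reachable points around its current location.
; RandomRoam3 starts on BeginPlay and calls itself again after each successful AI MoveTo, with no handling for failed moves.
; On seeing a pawn, PawnSensing issues an AI MoveTo with no destination or target set, then resumes roaming after a retriggerable delay.
; The graph contains no attack logic.
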(event OnSeePawn(PawnSensing)
  (params (Pawn :type Pawn%20Object%20Reference))
  (Utilities|FlowControl|Sequence
    (:then_0
      (AI|AIMoveTo self "0, 0, 0" 0 5.0 false))
    (:then_1
      (Utilities|FlowControl|RetriggerableDelay 1.0)
      (CallFunction|RandomRoam3))))

(event Custom|random_roam3
  (AI|AIMoveTo self (.RandomLocation (AI|Navigation|GetRandomReachablePointinRadius (Transformation|GetActorLocation) 0.0 0 0)) 0 5.0 false
    (:OnSuccess
      (CallFunction|RandomRoam3))))

(event EventBeginPlay
  (CallFunction|RandomRoam3))

(fn ConstructionScript)