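; Melee enemy NPC that chases the player and attacks on reaching them.
; Pawn sensing triggers FollowPlayer, which uses AI MoveTo toward the player, then plays a horizontal attack montage gated by a flag and a montage-length delay.
; Damage reduces health, stops the AI controller's brain logic at or below a threshold, and destroys the actor when health runs out.
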(event OnSeePawn(PawnSensing)
  (params (Pawn :type Pawn%20Object%20Reference))
  (Variables|Default|SetIsSeengPlayer true)
  (CallFunction|FollowPlayer))

(event Custom|FollowPlayer
  (Variables|Default|SetCanAtack true)
  (if (Variables|Default|GetIsSeengPlayer)
    (AI|AIMoveTo self "0, 0, 0" (Game|GetPlayerCharacter 0) 5.0 false
      (:OnSuccess
        (if (Variables|Default|GetCanAtack)
          (Variables|Default|SetCanAtack false)
          (bind _returnvalue (Animation|PlayAnimMontage "/Game/Briones/Animaciones/Standing_Melee_Attack_Horizontal_Anim_mixamo_com_Montage.Standing_Melee_Attack_Horizontal_Anim_mixamo_com_Montage" 1.0 "None"))
          (Utilities|FlowControl|Delay _returnvalue)
          (Variables|Default|SetCanAtack true))))))

(event Game|Damage|EventAnyDamage
  (params (Damage :type Float%20%28single-precision%29) (DamageType :type Damage%20Type%20Object%20Reference) (InstigatedBy :type Controller%20Object%20Reference) (DamageCauser :type Actor%20Object%20Reference))
  (bind _output_get (Variables|Default|SetHealtEnemy2 (- (Variables|Default|GetHealtEnemy2) Damage)))
  (if (<= _output_get 1e+04)
    (AI|Logic|StopLogic (Variables|/Script/AIModule.AIController|GetBrainComponent (AI|GetAIController self)) "")
    (if (<= _output_get 0.0)
      (Actor|DestroyActor))))

(fn ConstructionScript)