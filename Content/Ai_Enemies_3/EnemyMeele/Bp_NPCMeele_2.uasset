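; Melee enemy NPC, variant 2, that chases the player on sight and can be killed through damage.
; When PawnSensing sees any pawn, AIMoveTo targets player character 0, and the NPC destroys itself on reaching it, with no attack in this graph.
; Damage lowers HealtEnemy2, stopping the AI controller's brain logic at or below a threshold and destroying the actor at zero.
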(event OnSeePawn(PawnSensing)
  (params (Pawn :type Pawn%20Object%20Reference))
  (bind _asbp_third_person_character (Utilities|Casting|CastToBP_ThirdPersonCharacter (Game|GetPlayerCharacter 0)))
  (AI|AIMoveTo self "0, 0, 0" _asbp_third_person_character 5.0 false
    (:OnSuccess
      (Actor|DestroyActor))))

(event Game|Damage|EventAnyDamage
  (params (Damage :type Float%20%28single-precision%29) (DamageType :type Damage%20Type%20Object%20Reference) (InstigatedBy :type Controller%20Object%20Reference) (DamageCauser :type Actor%20Object%20Reference))
  (bind _output_get (Variables|Default|SetHealtEnemy2 (- (Variables|Default|GetHealtEnemy2) Damage)))
  (if (<= _output_get 1e+04)
    (AI|Logic|StopLogic (Variables|/Script/AIModule.AIController|GetBrainComponent (AI|GetAIController self)) "")
    (if (<= _output_get 0.0)
      (Actor|DestroyActor))))

(fn ConstructionScript)